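; Player 2 paddle for a Pong game, moved by physics impulses while W or S is held.
; The keys open a Gate that Tick feeds, pushing the paddle along X by the GetP2Moves axis value.
; Tick also checks upper and lower travel limits and calls the matching limit function.
; On BPIInteract it passes the ball's velocity to a force function and plays a collision sound if sound is enabled.
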(event EventBPIInteract
  (bind _ref_bp_ball (Variables|Default|GetRef%20BP%20Ball))
  (bind _ball (Variables|/Game/Blueprint/BP_Ball.BP_Ball_C|GetBall _ref_bp_ball))
  ;[1 1 1] BPI Ineraction With P2 Paddle
  (bind _returnvalue (Physics|GetPhysicsLinearVelocity _ball "None"))
  (CallFunction|FuncLBAddForcetoBall (Variables|Default|GetPaddleP2) _returnvalue _ball)
  (if (Variables|/Game/Blueprint/BP_PongGameInstance.BP_PongGameInstance_C|GetIsSoundOn? (Variables|Default|GetRef%20Game%20Instance))
    (Audio|PlaySoundatLocation "/Game/Sounds/S_ballCollision.S_ballCollision" "0, 0, 0" "0, 0, 0" 1.0 1.0 0.0 0 0 0)))

(event EventBeginPlay
  ;[1 1 1] Making Reference
  (bind _asbp_pong_game_instance (Utilities|Casting|CastToBP_PongGameInstance (Game|GetGameInstance)))
  (Variables|Default|SetRef%20Game%20Instance _asbp_pong_game_instance))

(event EventTick
  (params (DeltaSeconds :type Float%20%28single-precision%29))
  (Utilities|FlowControl|Sequence
    (:then_0
      ;[1 1 1] Moving Left Paddle Up And Down By Inputs W And S
      (Utilities|FlowControl|Gate true
        (:Exit
          (Physics|AddImpulse (Variables|Default|GetPaddleP2) (Math|Vector|MakeVector (* (Input|AxisValues|GetP2Moves) 3.5e+05) 0.0 0.0) "None" false))))
    (:then_1
      ;[1 1 1] Check If The AI Paddle Is At Highest And Or Lowest Place Prevent It From Moving More
      (if (CallFunction|UPLimitationCheck (Transformation|GetActorLocation))
        (CallFunction|FuncUpLimitation self (Transformation|GetActorLocation))
        (elif (CallFunction|DownLimitationCheck (Transformation|GetActorLocation))
          (CallFunction|FuncDownLimitation self (Transformation|GetActorLocation)))))))

(event Input|KeyboardEvents|W
  (params (Key :type Key%20Structure :default "None"))
  ;[1 1 1] Moving Left Paddle Up And Down By Inputs W And S
  (:Pressed
    (Utilities|FlowControl|Gate true) ; enters at Open
  )
  (:Released
    (Utilities|FlowControl|Gate true) ; enters at Close
  ))

(event Input|KeyboardEvents|S
  (params (Key :type Key%20Structure :default "None"))
  ;[1 1 1] Moving Left Paddle Up And Down By Inputs W And S
  (:Pressed
    (Utilities|FlowControl|Gate true) ; enters at Open
  )
  (:Released
    (Utilities|FlowControl|Gate true) ; enters at Close
  ))

(fn ConstructionScript)