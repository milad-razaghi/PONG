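; BP_Boundry is a Pong boundary that bounces the ball back when triggered through an interface interact event.
; On BeginPlay it caches the Pong game instance.
; BPIInteract negates the X component of the referenced ball's physics velocity, leaving Y and Z unchanged, then plays a collision sound if the game instance has sound enabled.
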(event EventBPIInteract
  (bind _ref_bp_ball (Variables|Default|GetRef_BP_Ball))
  (bind _ball (Variables|/Game/Blueprint/BP_Ball.BP_Ball_C|GetBall _ref_bp_ball))
  ;[1 1 1] BPI Event _If Boundries Overlaps With Ball Hitting It Back
  (bind _returnvalue (Physics|GetPhysicsLinearVelocity _ball "None"))
  (Physics|SetPhysicsLinearVelocity _ball (Math|Vector|MakeVector (* (.X (Math|Vector|BreakVector _returnvalue)) -1.0) (.Y (Math|Vector|BreakVector _returnvalue)) (.Z (Math|Vector|BreakVector _returnvalue))) false "None")
  (if (Variables|/Game/Blueprint/BP_PongGameInstance.BP_PongGameInstance_C|GetIsSoundOn? (Variables|Default|GetRef%20Game%20Instance))
    (Audio|PlaySoundatLocation "/Game/Sounds/S_ballCollision.S_ballCollision" "0, 0, 0" "0, 0, 0" 1.0 1.0 0.0 0 0 0)))

(event EventBeginPlay
  ;[1 1 1] Making reference
  (bind _asbp_pong_game_instance (Utilities|Casting|CastToBP_PongGameInstance (Game|GetGameInstance)))
  (Variables|Default|SetRef%20Game%20Instance _asbp_pong_game_instance))

(fn ConstructionScript)