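; Game instance for a Pong game that keeps the left and right scores and decides when a match ends.
; Two custom events add a point to a side and broadcast a dispatcher for that score change.
; The limit is checked before incrementing, so scoring again at five sets GameOver, broadcasts the win/lose result (true for right) and zeroes both scores.
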(event Custom|Cust_AddScoreToLeft
  ;[1 1 1] Check If It didn't Win Add Score To Left
  (if (>= (Variables|Default|GetLeftScore) 5)
    (Variables|Default|SetGameOver true)
    (Default|CallDispShowWinLose false)
    (Variables|Default|SetLeftScore 0)
    (Variables|Default|SetRightScore 0)
    (else
      (Variables|Default|SetLeftScore (+ (Variables|Default|GetLeftScore) 1))
      (Default|CallDispAddScoreL))))

(event Custom|Cust_AddScoreToRight
  ;[1 1 1] Check If It didn't Win Add Score To right
  (if (>= (Variables|Default|GetRightScore) 5)
    (Variables|Default|SetGameOver true)
    (Default|CallDispShowWinLose true)
    (Variables|Default|SetRightScore 0)
    (Variables|Default|SetLeftScore 0)
    (else
      (Variables|Default|SetRightScore (+ (Variables|Default|GetRightScore) 1))
      (Default|CallDispAddScoreR))))