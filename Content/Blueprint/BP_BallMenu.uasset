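; Menu-scene ball for a Pong game that also creates and shows the WBP_Menu widget on BeginPlay.
; After a short delay it launches with a diagonal physics velocity, then bounces on overlap by flipping X at BP_Boundry and Y at BP_Goal.
; Both bounces share a collision sound, played only when the cached BP_PongGameInstance has sound enabled.
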(event EventBeginPlay
  ;[1 1 1] Shooting Ball
  (Utilities|FlowControl|Sequence
    (:then_0
      (bind _returnvalue (UserInterface|CreateWidget "/Game/Blueprint/UI/WBP_Menu.WBP_Menu_C"))
      (bind _output_get (Variables|Default|SetRef%20WBP%20Menu _returnvalue))
      (UserInterface|Viewport|AddtoViewport _output_get 0))
    (:then_1
      (Utilities|FlowControl|Delay 0.2)
      (Physics|SetPhysicsLinearVelocity (Variables|Default|GetBall) "2000.000000,2000.000000, 0" false "None"))
    (:then_2
      (bind _asbp_pong_game_instance (Utilities|Casting|CastToBP_PongGameInstance (Game|GetGameInstance)))
      (Variables|Default|SetRef%20Game%20Instance _asbp_pong_game_instance))))

(event Collision|EventActorBeginOverlap
  (params (OtherActor :type Actor%20Object%20Reference))
  ;[1 1 1] If Pawn Overlaps With Ball Hitting It Back
  (Utilities|Casting|CastToBP_Boundry OtherActor
    (:then
      (bind _returnvalue (Physics|GetPhysicsLinearVelocity (Variables|Default|GetBall) "None"))
      (Physics|SetPhysicsLinearVelocity (Variables|Default|GetBall) (Math|Vector|MakeVector (* (.X (Math|Vector|BreakVector _returnvalue)) -1.0) (.Y (Math|Vector|BreakVector _returnvalue)) (.Z (Math|Vector|BreakVector _returnvalue))) false "None"))
    (:CastFailed
      (Utilities|Casting|CastToBP_Goal OtherActor)
      (bind _returnvalue_2 (Physics|GetPhysicsLinearVelocity (Variables|Default|GetBall) "None"))
      (Physics|SetPhysicsLinearVelocity (Variables|Default|GetBall) (Math|Vector|MakeVector (.X (Math|Vector|BreakVector _returnvalue_2)) (* (.Y (Math|Vector|BreakVector _returnvalue_2)) -1.0) (.Z (Math|Vector|BreakVector _returnvalue_2))) false "None")))
  (if (Variables|/Game/Blueprint/BP_PongGameInstance.BP_PongGameInstance_C|GetIsSoundOn? (Variables|Default|GetRef%20Game%20Instance))
    (Audio|PlaySoundatLocation "/Game/Sounds/S_ballCollision.S_ballCollision" "0, 0, 0" "0, 0, 0" 1.0 1.0 0.0 0 0 0)))

(fn ConstructionScript)