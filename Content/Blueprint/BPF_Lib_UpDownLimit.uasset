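; Blueprint function library of helpers that keep actors within upper and lower X limits and bounce a ball.
; The limit functions clamp an actor's X to the positive or negative half of the field, with matching checks for positions just beyond each outer edge.
; The bounce function overwrites the ball's physics velocity, combining the target's X velocity plus a random offset with the input vector's inverted Y and unchanged Z.
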(fn FuncUpLimitation
  (params (Target :type Actor%20Object%20Reference) (InVec :type Vector))
  (bind (_x _y _z) (Math|Vector|BreakVector InVec))
  (Transformation|SetActorLocation Target (Math|Vector|MakeVector (Math|Float|Clamp(Float) _x 0.0 1449.0) _y _z) false false))

(fn FuncDownLimitation
  (params (Target :type Actor%20Object%20Reference) (InVec :type Vector))
  (bind (_x _y _z) (Math|Vector|BreakVector InVec))
  (Transformation|SetActorLocation Target (Math|Vector|MakeVector (Math|Float|Clamp(Float) _x -1449.0 0.0) _y _z) false false))

(fn DownLimitationCheck
  (params (InVec :type Vector))
  (return (< (.X (Math|Vector|BreakVector InVec)) -1.45e+03)))

(fn UPLimitationCheck
  (params (InVec :type Vector))
  (return (> (.X (Math|Vector|BreakVector InVec)) 1.45e+03)))

(fn FuncLBAddForcetoBall
  (params (Target :type Primitive%20Component%20Object%20Reference) (InVec :type Vector) (BP%20Ball :type Primitive%20Component%20Object%20Reference))
  (bind (_x _y _z) (Math|Vector|BreakVector InVec))
  (bind _returnvalue (Physics|GetPhysicsLinearVelocity Target "None"))
  (Physics|SetPhysicsLinearVelocity BP%20Ball (Math|Vector|MakeVector (+ (.X (Math|Vector|BreakVector _returnvalue)) (Math|Random|RandomFloatinRange -1e+03 1e+03)) (* _y -1.0) _z) false "None")
  (return))