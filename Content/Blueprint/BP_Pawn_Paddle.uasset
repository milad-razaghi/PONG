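; Player 1's paddle pawn for a Pong game, moved by keyboard and able to hit the ball back.
; Up/Down keys open and close a Gate fed by Tick, applying an X-axis impulse scaled by the P1 movement input.
; Tick also uses function library helpers to enforce upper and lower travel limits.
; An interface event pushes the ball using its velocity and plays a collision sound when the GameInstance has sound enabled.
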(event EventBPIInteract
  (bind _ball (Variables|Default|GetBall))
  (bind _ball_2 (Variables|/Game/Blueprint/BP_Ball.BP_Ball_C|GetBall _ball))
  ;[1 1 1] BPI Event _If Paddle Overlaps With Ball Hitting It Back
  (bind _returnvalue (Physics|GetPhysicsLinearVelocity _ball_2 "None"))
  (CallFunction|FuncLBAddForcetoBall (Variables|Default|GetPaddle) _returnvalue _ball_2)
  (if (Variables|/Game/Blueprint/BP_PongGameInstance.BP_PongGameInstance_C|GetIsSoundOn? (Variables|Default|GetRef%20Game%20Instance))
    (Audio|PlaySoundatLocation "/Game/Sounds/S_ballCollision.S_ballCollision" "0, 0, 0" "0, 0, 0" 1.0 1.0 0.0 0 0 0)))

(event EventBeginPlay
  ;[1 1 1] Making reference
  (bind _asbp_pong_game_instance (Utilities|Casting|CastToBP_PongGameInstance (Game|GetGameInstance)))
  (Variables|Default|SetRef%20Game%20Instance _asbp_pong_game_instance))

(event EventTick
  (params (DeltaSeconds :type Float%20%28single-precision%29))
  ;[1 1 1] Controlling Limitation Of P1s' Moevement
  (Utilities|FlowControl|Sequence
    (:then_0
      (Utilities|FlowControl|Gate true
        (:Exit
          (Physics|AddImpulse (Variables|Default|GetPaddle) (Math|Vector|MakeVector (* (Input|AxisValues|GetP1Moves) 3.5e+05) 0.0 0.0) "None" false))))
    (:then_1
      (if (CallFunction|UPLimitationCheck (Transformation|GetActorLocation))
        (CallFunction|FuncUpLimitation self (Transformation|GetActorLocation)) ; Function Library
        (elif (CallFunction|DownLimitationCheck (Transformation|GetActorLocation))
          (CallFunction|FuncDownLimitation self (Transformation|GetActorLocation)) ; Function Library
        )))))

(event Input|KeyboardEvents|Up
  (params (Key :type Key%20Structure :default "None"))
  ;[1 1 1] Controlling Limitation Of P1s' Moevement
  (:Pressed
    (Utilities|FlowControl|Gate true) ; enters at Open
  )
  (:Released
    (Utilities|FlowControl|Gate true) ; enters at Close
  ))

(event Input|KeyboardEvents|Down
  (params (Key :type Key%20Structure :default "None"))
  ;[1 1 1] Controlling Limitation Of P1s' Moevement
  (:Pressed
    (Utilities|FlowControl|Gate true) ; enters at Open
  )
  (:Released
    (Utilities|FlowControl|Gate true) ; enters at Close
  ))

(fn ConstructionScript)