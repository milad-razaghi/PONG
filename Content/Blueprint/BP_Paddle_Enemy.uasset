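; BP_Paddle_Enemy is the AI opponent paddle in a Pong game.
; Each tick it tracks the ball along X with clamped physics impulses scaled by the GameMode's InterpolateTime.
; At either movement limit it calls a limitation function and zeroes its velocity instead.
; BPIInteract passes the ball's velocity to a force function and plays a collision sound if the GameInstance has sound enabled.
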(event EventBeginPlay
  ;[1 1 1] Making Reference
  (Utilities|FlowControl|Sequence
    (:then_0
      (bind _asbp_game_mode_pong (Utilities|Casting|CastToBP_GameModePong (Game|GetGameMode)))
      (Variables|Default|SetRef_GameMode _asbp_game_mode_pong))
    (:then_1
      (bind _asbp_pong_game_instance (Utilities|Casting|CastToBP_PongGameInstance (Game|GetGameInstance)))
      (Variables|Default|SetRef%20Game%20Instance _asbp_pong_game_instance))))

(event EventTick
  (params (DeltaSeconds :type Float%20%28single-precision%29))
  ;[1 1 1] Check If The AI Paddle Is At Highest And Or Lowest Place Prevent It From Moving More
  (if (CallFunction|UPLimitationCheck (Transformation|GetActorLocation))
    (CallFunction|FuncUpLimitation self (Transformation|GetActorLocation))
    (Physics|SetPhysicsLinearVelocity (Variables|Default|GetStaticMesh) "0, 0, 0" false "None")
    (elif (CallFunction|DownLimitationCheck (Transformation|GetActorLocation))
      (CallFunction|FuncDownLimitation self (Transformation|GetActorLocation))
      (Physics|SetPhysicsLinearVelocity (Variables|Default|GetStaticMesh) "0, 0, 0" false "None")
      (else
        (Physics|AddImpulse (Variables|Default|GetStaticMesh) (* (Math|Vector|MakeVector (Math|Float|Clamp(Float) (- (.X (Math|Vector|BreakVector (Transformation|GetActorLocation (Variables|Default|GetRef%20BP_Ball)))) (.X (Math|Vector|BreakVector (Transformation|GetActorLocation)))) -4.0 4.0) 0.0 0.0) (Variables|/Game/Blueprint/BP_GameModePong.BP_GameModePong_C|GetInterpolate%20Time (Variables|Default|GetRef_GameMode))) "None" false)))))

(event EventBPIInteract
  (bind _ref_bp_ball (Variables|Default|GetRef%20BP_Ball))
  (bind _ball (Variables|/Game/Blueprint/BP_Ball.BP_Ball_C|GetBall _ref_bp_ball))
  ;[1 0 0.7554] BPI Ineraction With Enemy Paddle
  (bind _returnvalue (Physics|GetPhysicsLinearVelocity _ball "None"))
  (CallFunction|FuncLBAddForcetoBall (Variables|Default|GetStaticMesh) _returnvalue _ball)
  (if (Variables|/Game/Blueprint/BP_PongGameInstance.BP_PongGameInstance_C|GetIsSoundOn? (Variables|Default|GetRef%20Game%20Instance))
    (Audio|PlaySoundatLocation "/Game/Sounds/S_ballCollision.S_ballCollision" "0, 0, 0" "0, 0, 0" 1.0 1.0 0.0 0 0 0)))

(fn ConstructionScript)