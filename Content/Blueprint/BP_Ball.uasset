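; Pong ball actor that serves from the world origin in a random left or right direction at BeginPlay.
; Two start events reset its position and set physics velocity, serving again after goals.
; Overlaps send an interface message to the other actor, so the ball needs no knowledge of its type.
; Tick polls GameOver on the cached Pong game instance and zeroes the ball's velocity once through a DoOnce.
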(event Custom|Cust_StartFromL
  ;[1 1 1] Strating Again (After Scoring Goal)
  (Transformation|SetActorLocation "0, 0, 0" false false)
  (Physics|SetPhysicsLinearVelocity (Variables|Default|GetBall) (Variables|Default|GetVelocityToRight) false "None"))

(event Custom|Cust_StartFromR
  ;[1 1 1] Strating Again (After Scoring Goal)
  (Transformation|SetActorLocation "0, 0, 0" false false)
  (Physics|SetPhysicsLinearVelocity (Variables|Default|GetBall) (Variables|Default|GetVelocityToLeft) false "None"))

(event Custom|Cust_GameOver
  ;[1 1 1] Check If Game Is Over Set The Ball location To zero
  (Utilities|FlowControl|DoOnce false
    (:Completed
      (Physics|SetPhysicsLinearVelocity (Variables|Default|GetBall) "0, 0, 0" false "None"))))

(event EventBeginPlay
  ;[1 1 1] Shooting Ball
  (Utilities|FlowControl|Sequence
    (:then_0
      (switch int (Math|Random|RandomIntegerinRange 0 1)
        (:0
          (CallFunction|CustStartfromL))
        (:1
          (CallFunction|CustStartfromR))))
    (:then_1
      (Utilities|IsValid (Variables|Default|GetRef%20GameINs)
        (:Is%20Not%20Valid
          (bind _asbp_pong_game_instance (Utilities|Casting|CastToBP_PongGameInstance (Game|GetGameInstance)))
          (Variables|Default|SetRef%20GameINs _asbp_pong_game_instance))))))

(event Collision|EventActorBeginOverlap
  (params (OtherActor :type Actor%20Object%20Reference))
  ;[0 0 1] Sending This Event To all Other Overlapping Actors By BP Interface Function
  (Class|BPIInteraction|BPIInteract(Message) OtherActor))

(event EventTick
  (params (DeltaSeconds :type Float%20%28single-precision%29))
  ;[1 1 1] Check If Game Is Over Set The Ball location To zero
  (if (Variables|/Game/Blueprint/BP_PongGameInstance.BP_PongGameInstance_C|GetGameOver (Variables|Default|GetRef%20GameINs))
    (CallFunction|CustGameOver)))

(fn ConstructionScript)