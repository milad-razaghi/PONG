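; Player controller for a Pong game that handles the quit prompt and restarting after game over.
; It caches the Pong game instance on BeginPlay to read and clear its GameOver flag.
; E or Escape pauses the game, shows the cursor, switches to UI-only input and opens the exit dialog widget.
; Space restarts the level through a console command, only when the game is over.
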(event EventBeginPlay
  (bind _asbp_pong_game_instance (Utilities|Casting|CastToBP_PongGameInstance (Game|GetGameInstance)))
  (Variables|Default|SetRef%20Game%20Instance _asbp_pong_game_instance))

(event Input|KeyboardEvents|Escape
  (params (Key :type Key%20Structure :default "None"))
  (bind _returnvalue (Game|GetPlayerController 0))
  ;[1 1 1] By Pressing Escape It's Gonna show Dialog box To Quit
  (:Pressed
    (Game|SetGamePaused true)
    (Variables|/Script/Engine.PlayerController|SetbShowMouseCursor _returnvalue true)
    (Input|SetInputModeUIOnly _returnvalue (stale _returnvalue_2) "DoNotLock")
    (bind _returnvalue_2 (UserInterface|CreateWidget "/Game/Blueprint/UI/WBP_ExitDialogBox.WBP_ExitDialogBox_C"))
    (UserInterface|Viewport|AddtoViewport _returnvalue_2 0)))

(event Input|KeyboardEvents|E
  (params (Key :type Key%20Structure :default "None"))
  (bind _returnvalue (Game|GetPlayerController 0))
  ;[1 1 1] By Pressing Escape It's Gonna show Dialog box To Quit
  (:Pressed
    (Game|SetGamePaused true)
    (Variables|/Script/Engine.PlayerController|SetbShowMouseCursor _returnvalue true)
    (Input|SetInputModeUIOnly _returnvalue (stale _returnvalue_2) "DoNotLock")
    (bind _returnvalue_2 (UserInterface|CreateWidget "/Game/Blueprint/UI/WBP_ExitDialogBox.WBP_ExitDialogBox_C"))
    (UserInterface|Viewport|AddtoViewport _returnvalue_2 0)))

(event Input|KeyboardEvents|SpaceBar
  (params (Key :type Key%20Structure :default "None"))
  (bind _ref_game_instance (Variables|Default|GetRef%20Game%20Instance))
  ;[1 1 1] Space Key To Restart
  (:Pressed
    (if (Variables|/Game/Blueprint/BP_PongGameInstance.BP_PongGameInstance_C|GetGameOver _ref_game_instance)
      (Development|ExecuteConsoleCommand "RestartLevel" 0)
      (Variables|/Game/Blueprint/BP_PongGameInstance.BP_PongGameInstance_C|SetGameOver _ref_game_instance false))))

(fn ConstructionScript)