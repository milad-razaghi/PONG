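; Goal actor for a Pong game that handles scoring when it receives the BPI interact event, intended for the ball hitting a goal.
; Its GateSide value decides which player scores: the game instance, cached on BeginPlay, adds a point to the side opposite the goal.
; It then restarts the referenced ball through a side-specific custom event and plays a goal sound if sound is enabled in the game instance.
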(event EventBeginPlay
  ;[1 1 1] Making Reference To Game Mode
  (bind _asbp_pong_game_instance (Utilities|Casting|CastToBP_PongGameInstance (Game|GetGameInstance)))
  (Variables|Default|SetRef%20Game%20Instance _asbp_pong_game_instance))

(event EventBPIInteract
  ;[1 1 1] BPI Event Interacting Ball With Goals
  (Utilities|FlowControl|Sequence
    (:then_0
      (if (Utilities|Enum|Equal(Enum) (Variables|Default|GetGateSide) (Variables|Default|GetLeftGoal))
        (Default|CustAddScoretoRight (Variables|Default|GetRef%20Game%20Instance))
        (Default|CustStartfromR (Variables|Default|GetRef_BP%20Ball)) ; The Left One Recieved Goal Start To Left
        (if (Variables|/Game/Blueprint/BP_PongGameInstance.BP_PongGameInstance_C|GetIsSoundOn? (Variables|Default|GetRef%20Game%20Instance)) :!label _label
          (Audio|SpawnSoundatLocation "/Game/Sounds/S_ballGoal.S_ballGoal" "0,0.000000, 0" "0, 0, 0" 1.0 1.0 0.0 0 0))))
    (:then_1
      (if (Utilities|Enum|Equal(Enum) (Variables|Default|GetGateSide) (Variables|Default|GetRightGoal))
        (Default|CustAddScoretoLeft (Variables|Default|GetRef%20Game%20Instance))
        (Default|CustStartfromL (Variables|Default|GetRef_BP%20Ball)) ; The Left One Recieved Goal Start To Left
        (goto _label)))))

(fn ConstructionScript)